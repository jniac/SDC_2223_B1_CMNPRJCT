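; Checkpoint actor shown as a bobbing, spinning torus that registers itself with an overlapping sdc_BP_Character and exposes an Arrow as spawn transform.
; Activate and Deactivate only set a flag, which picks the direction in which Tick manually scrubs two timelines, so transitions reverse smoothly.
; The short timeline blends the torus from sine bobbing to a raised, enlarged pose, and the regular one drives a material Fill parameter.
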(event EventDeactivateCheckpoint
  (Variables|Default|Setactivated false))

(event EventActivateCheckpoint
  (Variables|Default|Setactivated true))

(event Collision|EventActorBeginOverlap
  (params (OtherActor :type Actor%20Object%20Reference))
  (bind _assdc_bp_character (Utilities|Casting|CastTosdc_BP_Character OtherActor))
  (Default|SetCheckPoint _assdc_bp_character self))

(event EventTick
  (params (DeltaSeconds :type Float%20%28single-precision%29))
  (CallFunction|UpdateTime DeltaSeconds)
  (CallFunction|UpdateTorus))

(fn ConstructionScript
  (Variables|Default|SetinitialTorusZ (.z (Variables|/Script/Engine.SceneComponent|GetRelativeLocation (Variables|Transformation|GetTorus)))))

(fn UpdateTorus
  (bind _activationshort (Variables|Default|GetactivationShort))
  (bind _time (Variables|Default|Gettime))
  (bind _returnvalue (Math|Float|Lerp 1.0 1.2 _activationshort))
  (Transformation|SetRelativeLocation (Variables|Transformation|GetTorus) (Math|Vector|MakeVector 0.0 0.0 (Math|Float|Lerp (CallFunction|GetTorusSinY) (+ (Variables|Default|GetinitialTorusZ) 1e+02) (Variables|Default|GetactivationShort))) false false)
  (Transformation|SetRelativeScale3D (Variables|Transformation|GetTorus) (Math|Vector|MakeVector _returnvalue _returnvalue _returnvalue))
  (Transformation|SetRelativeRotation (Variables|Transformation|GetTorus) (Math|Rotator|MakeRotator 0.0 (* _time 9e+01) (* _time 3e+01)) false false))

(fn UpdateTime
  (params (deltaSeconds :type Float%20%28double-precision%29))
  (bind _returnvalue (* deltaSeconds -1.0))
  (bind _activated (Variables|Default|Getactivated))
  (bind _returnvalue_2 (Math|Float|SelectFloat deltaSeconds _returnvalue _activated))
  (Variables|Default|Settime (+ (Variables|Default|Gettime) deltaSeconds))
  (CallFunction|UpdateTimelinePlayback (Variables|Default|GetActivationShortTimeline) _returnvalue_2)
  (CallFunction|UpdateTimelinePlayback (Variables|Default|GetActivationRegularTimeline) _returnvalue_2))

(fn GetTorusSinY
  (return (+ (* (Math|Trig|Sin(Radians) (* (Variables|Default|Gettime) 1.0)) 1e+01) (Variables|Default|GetinitialTorusZ))))

(fn UpdateTimelinePlayback
  (params (timeline :type Timeline%20Component%20Object%20Reference) (deltaSeconds :type Float%20%28double-precision%29))
  (Components|Timeline|SetPlaybackPosition timeline (Math|Float|Clamp(Float) (+ (Components|Timeline|GetPlaybackPosition timeline) deltaSeconds) 0.0 (Components|Timeline|GetTimelineLength timeline)) true true))

(fn GetSpawnTransform
  (return (Transformation|GetWorldTransform (Variables|Default|GetArrow))))